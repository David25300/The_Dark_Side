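; First-person player character Blueprint handling movement, look, jump, crouch and sprint input.
; Crouch toggles through a FlipFlop, with a reversible timeline blending capsule half-height and camera boom height.
; Holding sprint drives a second timeline blending walk speed and camera FOV, with press and release both ignored while crouched.
; Every tick starts an idle or walk/run camera shake on the player camera manager, chosen by velocity.
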(event Custom|Camera%20Shake%20Event
  (bind _returnvalue (Game|GetPlayerCameraManager 0))
  ;[1 1 1] Camera Shake
  (if (<= (Math|Vector|VectorLength (Transformation|GetVelocity)) 0.0)
    (Class|PlayerCameraManager|StartMatineeCameraShakefromSource _returnvalue "/Game/cAMERa/Camera-Shake-Idle.Camera-Shake-Idle_C" 0 1.0 "CameraLocal" "0, 0, 0")
    (else
      (Class|PlayerCameraManager|StartMatineeCameraShakefromSource _returnvalue "/Game/cAMERa/Camera-Shake-Walk-Run.Camera-Shake-Walk-Run_C" 0 1.0 "CameraLocal" "0, 0, 0"))))

(event EventTick
  (params (DeltaSeconds :type Float%20%28single-precision%29))
  ;[1 1 1] Event Tick
  (CallFunction|CameraShakeEvent))

(event Input|ActionEvents|InputActionSalto
  (params (Key :type Key%20Structure :default "None"))
  ;[1 1 1] Salto
  (:Pressed
    (Character|Jump)))

(event Input|ActionEvents|InputActionAgacharse
  (params (Key :type Key%20Structure :default "None"))
  ;[1 1 1] Agachardito
  (:Pressed
    (Utilities|FlowControl|FlipFlop
      (:A
        (Variables|Default|SetAgachado? true))
      (:B
        (Variables|Default|SetAgachado? false)))
    (if (Variables|Default|GetAgachado?)
      (bind _newtrack_0 (Timeline|Agachado Play)
        (:Update
          (Components|Capsule|SetCapsuleHalfHeight (Variables|Collision|GetCapsuleComponent) (Math|Float|Lerp 88.0 58.0 _newtrack_0) true)
          (Transformation|SetRelativeLocation (Variables|Default|GetCameraBoom) (Math|Vector|MakeVector 0.0 0.0 (Math|Float|Lerp 49.0 2e+01 _newtrack_0)) false false)))
      (else
        (Timeline|Agachado Reverse)))))

(event Input|ActionEvents|InputActionCorrer
  (params (Key :type Key%20Structure :default "None"))
  (bind _agachado_ (Variables|Default|GetAgachado?))
  ;[1 1 1] Correr
  (:Pressed
    (if (not _agachado_)
      (Variables|Default|SetCorriendo? true)
      (if (Variables|Default|GetCorriendo?) :!label _label
        (bind _tiempo_de_correr (Timeline|Línea%20de%20tiempo_0 Play)
          (:Update
            (Variables|/Script/Engine.CharacterMovementComponent|SetMaxWalkSpeed (Variables|Character|GetCharacterMovement) (Math|Float|Lerp 3e+02 6e+02 _tiempo_de_correr))
            (Camera|SetFieldOfView (Variables|Default|GetCamera) (Math|Float|Lerp 9e+01 1.1e+02 _tiempo_de_correr))))
        (else
          (Timeline|Línea%20de%20tiempo_0 Reverse)))))
  (:Released
    (if (not _agachado_)
      (Variables|Default|SetCorriendo? false)
      (goto _label))))

(event Input|AxisEvents|InputAxisMDerecha
  (params (AxisValue :type Float%20%28single-precision%29))
  ;[1 1 1] Movimiento input
  (Pawn|Input|AddMovementInput (Math|Vector|GetRightVector (Math|Rotator|MakeRotator 0.0 0.0 (.yaw (Pawn|GetControlRotation :!class /Script/Engine.Pawn)))) AxisValue false))

(event Input|AxisEvents|InputAxisMDelante
  (params (AxisValue :type Float%20%28single-precision%29))
  ;[1 1 1] Movimiento input
  (Pawn|Input|AddMovementInput (Math|Vector|GetForwardVector (Math|Rotator|MakeRotator 0.0 0.0 (.yaw (Pawn|GetControlRotation :!class /Script/Engine.Pawn)))) AxisValue false))

(event Input|AxisEvents|InputAxisLookUp
  (params (AxisValue :type Float%20%28single-precision%29))
  ;[1 1 1] Movimiento input
  (Pawn|Input|AddControllerPitchInput (* AxisValue 1.0)))

(event Input|AxisEvents|InputAxisLookRigth
  (params (AxisValue :type Float%20%28single-precision%29))
  ;[1 1 1] Movimiento input
  (Pawn|Input|AddControllerYawInput (* AxisValue 1.0)))

(fn ConstructionScript)